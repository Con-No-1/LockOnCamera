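; Actor component that locks its owning Character's spring arm and camera onto the nearest actor with an enabled AC_LockOnTarget component.
; Each tick it scans all actors, honoring each target's optional auto-enable distance, and picks the closest.
; It then snaps or interpolates both components toward it, using per-target overrides when set.
; While locked it disables pawn control rotation, restoring that and saved relative rotations when no targets remain.
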(event `self.ReceiveBeginPlay`
  ;[1 1 1] Set Owner, Spring Arm, and Camera.
  (`|ExecutionSequence`
    (:`then_0`
      (bind _ascharacter (cast `Character` (`self.GetOwner`)))
      (set `self.Owning Character` _ascharacter)
      (set `self.Spring Arm` (`Actor.GetComponentByClass` (`self.Owning Character`) "/Script/Engine.SpringArmComponent"))
      (set `self.Camera` (`Actor.GetComponentByClass` (`self.Owning Character`) "/Script/Engine.CameraComponent"))
      (bind _camera (`self.Camera`)
        (:`then`
          (set `self.Camera Use Pawn Control Rotation` (`CameraComponent.bUsePawnControlRotation` _camera)))
        (:`else`
          (`KismetSystemLibrary.PrintText` "ERROR: Add a Camera to AC_LockOnCamera Character" true true (struct :`R` 1.0 :`A` 1.0) 5.0)))
      (bind _spring_arm (`self.Spring Arm`)
        (:`then`
          (set `self.Spring Use Pawn Control Rotation` (`SpringArmComponent.bUsePawnControlRotation` _spring_arm)))
        (:`else`
          (`KismetSystemLibrary.PrintText` "ERROR: Add a Spring Arm to AC_LockOnCamera Character" true true (struct :`R` 1.0 :`A` 1.0) 5.0))))
    (:`then_1`
      (`self.Set Reset Camera Rotation`))))

(event `Set Reset Camera Rotation`
  ;[0.5 1 0.5] Set what the rotations of camera and spring arm will be when there are no targets
  (`|ExecutionSequence`
    (:`then_0`
      (bind _spring_arm (`self.Spring Arm`)
        (:`then`
          (set `self.Spring Arm Reset Rotation` (`SceneComponent.RelativeRotation` _spring_arm)))
        (:`else`)))
    (:`then_1`
      (bind _camera (`self.Camera`)
        (:`then`
          (set `self.Camera Reset Rotation` (`SceneComponent.RelativeRotation` _camera)))
        (:`else`)))))

(event `Reset Camera Rotation`
  ;[0.25 1 0.25] Set the rotations of camera and spring arm when there are no targets
  (`|ExecutionSequence`
    (:`then_0`
      (bind _spring_arm (`self.Spring Arm`)
        (:`then`
          (`SceneComponent.K2_SetRelativeRotation` _spring_arm (`self.Spring Arm Reset Rotation`) false false))
        (:`else`)))
    (:`then_1`
      (bind _camera (`self.Camera`)
        (:`then`
          (`SceneComponent.K2_SetRelativeRotation` _camera (`self.Camera Reset Rotation`) false false))
        (:`else`)))))

(event `self.ReceiveTick`
  (params (DeltaSeconds :type "Float (single-precision)"))
  (bind _returnvalue (`Actor.GetComponentByClass` (`self.Target`) "/Lock-OnCameraAndMiscTools/AC_LockOnTarget.AC_LockOnTarget_C"))
  (bind _returnvalue_2 (`KismetMathLibrary.FindLookAtRotation` (`SceneComponent.K2_GetComponentLocation` (`self.Camera`)) (`SceneComponent.K2_GetComponentLocation` (`Actor.RootComponent` (`self.Target`)))))
  (bind _returnvalue_3 (`KismetMathLibrary.RInterpTo` (`SceneComponent.K2_GetComponentRotation` (`self.Camera`)) (`KismetMathLibrary.FindLookAtRotation` (`SceneComponent.K2_GetComponentLocation` (`self.Camera`)) (`SceneComponent.K2_GetComponentLocation` (`Actor.RootComponent` (`self.Target`)))) (`self.Delta Time`) (`/Lock-OnCameraAndMiscTools/AC_LockOnTarget.Interpolation Speed` (`Actor.GetComponentByClass` (`self.Target`) "/Lock-OnCameraAndMiscTools/AC_LockOnTarget.AC_LockOnTarget_C"))))
  (bind _returnvalue_4 (`KismetMathLibrary.RInterpTo` (`SceneComponent.K2_GetComponentRotation` (`self.Camera`)) (`KismetMathLibrary.FindLookAtRotation` (`SceneComponent.K2_GetComponentLocation` (`self.Camera`)) (`SceneComponent.K2_GetComponentLocation` (`Actor.RootComponent` (`self.Target`)))) (`self.Delta Time`) (`self.Interpolate Speed`)))
  ;[0.5 0.5 1] Rotates Camera to Target every frame (If target is valid)
  (set `self.Delta Time` DeltaSeconds)
  (`self.Get Target`)
  (`self.Target`
    (:`then`
      (if (`/Lock-OnCameraAndMiscTools/AC_LockOnTarget.Enabled` (`Actor.GetComponentByClass` (`self.Target`) "/Lock-OnCameraAndMiscTools/AC_LockOnTarget.AC_LockOnTarget_C"))
        (if (`/Lock-OnCameraAndMiscTools/AC_LockOnTarget.Override Lock on Type` _returnvalue)
          (switch `/Lock-OnCameraAndMiscTools/Enum_LockOnType` (`/Lock-OnCameraAndMiscTools/AC_LockOnTarget.Lock on Type` _returnvalue)
            (:`NewEnumerator0`
              (bind _spring_arm (`self.Spring Arm` :!label _label)
                (:`then`
                  (`SceneComponent.K2_SetWorldRotation` _spring_arm _returnvalue_2 false false)
                  (bind _camera (`self.Camera`)
                    (:`then`
                      (`SceneComponent.K2_SetWorldRotation` _camera _returnvalue_2 false false))
                    (:`else`
                      (`KismetSystemLibrary.PrintString` "No Valid Camera"))))
                (:`else`
                  (`KismetSystemLibrary.PrintString` "No Valid Spring Arm"))))
            (:`NewEnumerator1`
              (if (`/Lock-OnCameraAndMiscTools/AC_LockOnTarget.Override Interpolation Speed` (`Actor.GetComponentByClass` (`self.Target`) "/Lock-OnCameraAndMiscTools/AC_LockOnTarget.AC_LockOnTarget_C")) :!label _label_2
                (bind _spring_arm_2 (`self.Spring Arm`)
                  (:`then`
                    (`SceneComponent.K2_SetWorldRotation` _spring_arm_2 _returnvalue_3 false false)
                    (bind _camera_2 (`self.Camera`)
                      (:`then`
                        (`SceneComponent.K2_SetWorldRotation` _camera_2 _returnvalue_3 false false))
                      (:`else`
                        (`KismetSystemLibrary.PrintString` "No Valid Camera"))))
                  (:`else`
                    (`KismetSystemLibrary.PrintString` "No Valid Spring Arm")))
                (else
                  (bind _spring_arm_3 (`self.Spring Arm`)
                    (:`then`
                      (`SceneComponent.K2_SetWorldRotation` _spring_arm_3 _returnvalue_4 false false)
                      (bind _camera_3 (`self.Camera`)
                        (:`then`
                          (`SceneComponent.K2_SetWorldRotation` _camera_3 _returnvalue_4 false false))
                        (:`else`
                          (`KismetSystemLibrary.PrintString` "No Valid Camera"))))
                    (:`else`
                      (`KismetSystemLibrary.PrintString` "No Valid Spring Arm")))))))
          (else
            (switch `/Lock-OnCameraAndMiscTools/Enum_LockOnType` (`self.Lock On Type`)
              (:`NewEnumerator0`
                (goto _label))
              (:`NewEnumerator1`
                (goto _label_2)))))))
    (:`else`)))

(event `Get Target`
  ;[1 0.5 0.5] Set Camera Target to nearest valid target
  (set `self.Target` null)
  (set `self.Temp Target` null)
  (bind _outactors (`GameplayStatics.GetAllActorsOfClass` "/Script/Engine.Actor"))
  (for _array_element _outactors
    (if (`self.Is Camera Lock Enabled?` _array_element)
      (`/Engine/EditorBlueprintResources/StandardMacros.IncrementInt` (`self.No of Valid Targets`)
        (:`  `
          (set `self.Temp Target` _array_element)
          (if (or (< (`Actor.GetDistanceTo` (`self.Owning Character`) (`self.Temp Target`)) (`Actor.GetDistanceTo` (`self.Owning Character`) (`self.Target`))) (not (`KismetSystemLibrary.IsValid` (`self.Target`))))
            (set `self.Target` _array_element))))))
  (`|ExecutionSequence`
    (:`then_0`
      (if (== (`self.No of Valid Targets`) 0)
        (if (`self.Had Target Since Rotation Reset`)
          (`self.Reset Camera Rotation`))
        (`self.Set Reset Camera Rotation`)
        (set `self.Had Target Since Rotation Reset` false)
        (bind _camera (`self.Camera`)
          (:`then`
            (set `CameraComponent.bUsePawnControlRotation` (`self.Camera Use Pawn Control Rotation`) _camera)
            (bind _spring_arm (`self.Spring Arm`)
              (:`then`
                (set `SpringArmComponent.bUsePawnControlRotation` (`self.Spring Use Pawn Control Rotation`) _spring_arm))
              (:`else`)))
          (:`else`))
        (else
          (set `self.Had Target Since Rotation Reset` true)
          (`self.Camera`
            (:`then`
              (set `CameraComponent.bUsePawnControlRotation` false _camera)
              (`self.Spring Arm`
                (:`then`
                  (set `SpringArmComponent.bUsePawnControlRotation` false _spring_arm))
                (:`else`)))
            (:`else`)))))
    (:`then_1`
      (set `self.No of Valid Targets` 0))))

(fn `Is Camera Lock Enabled?`
  (params (`Target Actor` :type "Actor Object Reference"))
  (returns (Enabled :type Boolean))
  (bind _returnvalue (`Actor.GetComponentByClass` `Target Actor` "/Lock-OnCameraAndMiscTools/AC_LockOnTarget.AC_LockOnTarget_C"))
  (`/Engine/EditorBlueprintResources/StandardMacros.IsValid` _returnvalue
    (:`Is Valid`
      (if (`/Lock-OnCameraAndMiscTools/AC_LockOnTarget.Enabled` _returnvalue)
        (if (`/Lock-OnCameraAndMiscTools/AC_LockOnTarget.Auto-Enable by Distance` _returnvalue)
          (if (<= (`Actor.GetDistanceTo` (`self.Owning Character`) `Target Actor`) (`/Lock-OnCameraAndMiscTools/AC_LockOnTarget.Auto-Enable Distance` _returnvalue))
            (return true)
            (else
              (return false)))
          (else
            (return true)))
        (else
          (return false))))
    (:`Is Not Valid`
      (return false))))