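; Actor component that locks the owner's camera onto the nearest actor with an enabled AC_LockOnTarget component.
; A looping timer periodically scans every actor in the world to pick that target, with no range or visibility check.
; Each Tick turns the owner's spring arm and camera toward the target's root, either snapping or interpolating according to LockOnType.
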(event `self.ReceiveBeginPlay`
  (`|ExecutionSequence`
    (:`then_0`
      (set `self.Owning Actor` (`self.GetOwner`))
      (set `self.Spring Arm` (`Actor.GetComponentByClass` (`self.Owning Actor`) "/Script/Engine.SpringArmComponent"))
      (set `self.Camera` (`Actor.GetComponentByClass` (`self.Owning Actor`) "/Script/Engine.CameraComponent")))
    (:`then_1`
      (`self.Get Target Loop`))))

(event `self.ReceiveTick`
  (params (DeltaSeconds :type "Float (single-precision)"))
  (bind _returnvalue (`KismetMathLibrary.FindLookAtRotation` (`SceneComponent.K2_GetComponentLocation` (`self.Camera`)) (`SceneComponent.K2_GetComponentLocation` (`Actor.RootComponent` (`self.Target`)))))
  (bind _returnvalue_2 (`KismetMathLibrary.RInterpTo` (`SceneComponent.K2_GetComponentRotation` (`self.Camera`)) (`KismetMathLibrary.FindLookAtRotation` (`SceneComponent.K2_GetComponentLocation` (`self.Camera`)) (`SceneComponent.K2_GetComponentLocation` (`Actor.RootComponent` (`self.Target`)))) (`self.Delta Time`) (`self.Interpolate Speed`)))
  (set `self.Delta Time` DeltaSeconds)
  (`self.Target`
    (:`then`
      (if (`/Lock-OnCameraAndMiscTools/AC_LockOnTarget.Enabled` (`Actor.GetComponentByClass` (`self.Target`) "/Lock-OnCameraAndMiscTools/AC_LockOnTarget.AC_LockOnTarget_C"))
        (switch `/Lock-OnCameraAndMiscTools/Enum_LockOnType` (`self.Lock On Type`)
          (:`NewEnumerator0`
            (`|ExecutionSequence`
              (:`then_0`
                (bind _spring_arm (`self.Spring Arm`)
                  (:`then`
                    (`SceneComponent.K2_SetWorldRotation` _spring_arm _returnvalue false false))
                  (:`else`)))
              (:`then_1`
                (bind _camera (`self.Camera`)
                  (:`then`
                    (`SceneComponent.K2_SetWorldRotation` _camera _returnvalue false false))
                  (:`else`
                    (`KismetSystemLibrary.PrintString` "No Valid Camera"))))))
          (:`NewEnumerator1`
            (`|ExecutionSequence`
              (:`then_0`
                (bind _spring_arm_2 (`self.Spring Arm`)
                  (:`then`
                    (`SceneComponent.K2_SetWorldRotation` _spring_arm_2 _returnvalue_2 false false))
                  (:`else`)))
              (:`then_1`
                (bind _camera_2 (`self.Camera`)
                  (:`then`
                    (`SceneComponent.K2_SetWorldRotation` _camera_2 _returnvalue_2 false false))
                  (:`else`
                    (`KismetSystemLibrary.PrintString` "No Valid Camera")))))))))
    (:`else`)))

(event `Get Target Loop`
  (`KismetSystemLibrary.K2_SetTimerDelegate` (delegate `Get Target`) 0.1 true true))

(event `Get Target`
  (set `self.Target` null)
  (set `self.Temp Target` null)
  (bind _outactors (`GameplayStatics.GetAllActorsOfClass` "/Script/Engine.Actor"))
  (for _array_element _outactors
    (bind _returnvalue (`Actor.GetComponentByClass` _array_element "/Lock-OnCameraAndMiscTools/AC_LockOnTarget.AC_LockOnTarget_C"))
    (`/Engine/EditorBlueprintResources/StandardMacros.IsValid` _returnvalue
      (:`Is Valid`
        (if (`/Lock-OnCameraAndMiscTools/AC_LockOnTarget.Enabled` _returnvalue)
          (set `self.Temp Target` _array_element)
          (if (or (< (`Actor.GetDistanceTo` (`self.Owning Actor`) (`self.Temp Target`)) (`Actor.GetDistanceTo` (`self.Owning Actor`) (`self.Target`))) (not (`KismetSystemLibrary.IsValid` (`self.Target`))))
            (set `self.Target` _array_element)))))))